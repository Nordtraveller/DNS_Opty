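; BP_Spawner fills the level with a grid of a configurable skeletal actor class, likely for LOD testing.
; SpawnSkeletals first destroys every SkeletalMeshActor in the level, then loops rows and columns to spawn actors at a set spacing.
; The grid centers roughly on the world origin, independent of the spawner's transform, and spawning ignores collisions.
; The event graph and construction script are empty, so nothing here calls SpawnSkeletals.
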(event EventBeginPlay)

(event Collision|EventActorBeginOverlap
  (params (OtherActor :type Actor%20Object%20Reference)))

(event EventTick
  (params (DeltaSeconds :type Float%20%28single-precision%29)))

(fn ConstructionScript)

(fn SpawnSkeletals
  (bind _numberofrows (Variables|Spawn|GetNumberOfRows))
  (bind _numberofcolumns (Variables|Spawn|GetNumberOfColumns))
  ;[1 1 1] Cleanup off old actors
  (bind _outactors (Actor|GetAllActorsOfClass "/Script/Engine.SkeletalMeshActor"))
  (for _array_element _outactors
    (Actor|DestroyActor _array_element))
  (for _index (range 0 _numberofrows)
    (for _index_2 (range 0 _numberofcolumns)
      (Game|SpawnActorfromClass (Variables|Spawn|GetSkeletalToSpawn) (Math|Transform|MakeTransform (Math|Vector|MakeVector (* (- _index_2 (/ _numberofcolumns 2)) (Variables|Spawn|GetDistanceUnit)) (* (- _index (/ _numberofrows 2)) (Variables|Spawn|GetDistanceUnit)) 0.0)) "AlwaysSpawn" 0 0))))